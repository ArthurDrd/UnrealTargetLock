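; HUD Blueprint that displays a crosshair widget at the center of the owning player's viewport.
; BeginPlay creates WBP_Crosshair, adds it to the viewport and centers it using half the viewport size with DPI scale removed.
; DrawHUD repeats the centering on every draw, so the crosshair follows viewport size changes.
; The SetCrosshairPosition event is an empty stub.
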(event `self.ReceiveBeginPlay`
  (`parent.ReceiveBeginPlay`)
  (bind _returnvalue (`|CreateWidget` "/Game/Game/Blueprints/WBP/WBP_Crosshair.WBP_Crosshair_C"))
  (bind _output_get (set `self.WBP Crosshair` _returnvalue))
  (`UserWidget.AddToViewport` _output_get 0)
  (`self.SetDefaultCrosshairPosition`))

(event `self.SetCrosshairPosition`
  (params (ScreenPosition :type "Vector2D Structure (by ref)")))

(event `self.SetDefaultCrosshairPosition`
  (bind (_sizex _sizey) (`PlayerController.GetViewportSize` (`self.GetOwningPlayerController`)))
  (`UserWidget.SetPositionInViewport` (`self.WBP Crosshair`) (`KismetMathLibrary.MakeVector2D` (`KismetMathLibrary.Conv_IntToDouble` (/ _sizex 2)) (`KismetMathLibrary.Conv_IntToDouble` (/ _sizey 2))) true))

(event `self.ReceiveDrawHUD`
  (params (SizeX :type Integer) (SizeY :type Integer))
  (`self.SetDefaultCrosshairPosition`))

(fn `UserConstructionScript`)